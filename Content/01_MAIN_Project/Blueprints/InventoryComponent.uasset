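; Actor component that stores an inventory as a slot array and toggles its on-screen window.
; BeginPlay sizes the array to the slot count, and adding writes contents into the first default-valued slot, without merging stacks, and always reports success.
; Toggling either removes the window and restores game input, or creates it on the player controller's HUD canvas with center anchors and switches to UI-only input.
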(event EventBeginPlay
  (CallFunction|PrepareInventory))

(event EventTick
  (params (DeltaSeconds :type Float%20%28single-precision%29)))

(fn ToggleInventory
  (Variables|Default|GetInventoryWindow
    (:then
      (Widget|RemovefromParent (Variables|Default|GetInventoryWindow))
      (Variables|Default|SetInventoryWindow 0)
      (Input|SetInputModeGameOnly (Game|GetPlayerController 0)))
    (:else
      (bind _returnvalue (UserInterface|CreateWidget "/Game/01_MAIN_Project/UI/InventoryUI/InventoryWindow.InventoryWindow_C" 0 self))
      (Variables|Default|SetInventoryWindow _returnvalue)
      (bind _asmy_player_controller (Utilities|Casting|CastToMyPlayerController (Game|GetPlayerController 0)))
      (bind _returnvalue_2 (Class|CanvasPanel|AddChildtoCanvas (Variables|/Game/01_MAIN_Project/UI/InventoryUI/HUD.HUD_C|GetHud_canvas (Variables|/Game/01_MAIN_Project/Blueprints/MyPlayerController.MyPlayerController_C|Gethud_widget _asmy_player_controller)) (Variables|Default|GetInventoryWindow)))
      (Class|CanvasPanelSlot|SetAutoSize _returnvalue_2 true)
      (Class|CanvasPanelSlot|SetAlignment _returnvalue_2 "(X=0.500000,Y=0.500000)")
      (Class|CanvasPanelSlot|SetAnchors _returnvalue_2 (Utilities|Struct|MakeAnchors "(X=0.500000,Y=0.500000)" "(X=0.500000,Y=0.500000)"))
      (Class|CanvasPanelSlot|SetPosition _returnvalue_2 (Variables|Default|Getposition))
      (Input|SetInputModeUIOnly (Game|GetPlayerController 0) (Variables|Default|GetInventoryWindow) "LockAlways"))))

(fn AddtoInventory
  (params (ContentsToAdd :type Slot%20Structure%20Structure))
  (CallFunction|CreateStack ContentsToAdd)
  (return true))

(fn PrepareInventory
  (Utilities|Array|Resize (Variables|Default|GetInventory) (Variables|Default|GetNumberOfSlots)))

(fn CreateStack
  (params (ContenttoAdd :type Slot%20Structure%20Structure))
  (bind _inventory (Variables|Default|GetInventory))
  (Utilities|Array|SetArrayElem _inventory (Utilities|Array|FindItem _inventory (Utilities|Struct|MakeSlotStructure "(Name_3_F421C9994409CA97B694C68FB9A08C0E=NSLOCTEXT(\"[A4B82BEB4B3BFA6383493F9970285480]\", \"B7E515594E3AB67CA92E249E63A6B6C9\", \"None\"),Thumbnail_5_1173753A4AD7E44866616A8A8C2ACBD5=None,Description_8_707625D84A895ABF34D29A881E5949F2=NSLOCTEXT(\"[A4B82BEB4B3BFA6383493F9970285480]\", \"EC54E575421B4B482848B08D02E6B494\", \"None\"),Item_11_2C54BC0744A494098329BBA7F728A928=None)")) ContenttoAdd))